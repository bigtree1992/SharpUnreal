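; A test pawn with three-axis movement, Level Sequence event hooks and VR motion controller input logging.
; Movement axes each keep only one control rotation component around their own axis, so input resolves to fixed world directions.
; BeginPlay registers the pawn as event receiver on the first LevelSequenceActor found, whose events one, two and three print their names.
; Trigger and grip presses print Chinese debug labels; the sequence Play call is unconnected.
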(event Custom|one
  (Development|PrintString "one"))

(event Custom|two
  (Development|PrintString "two"))

(event Custom|three
  (Development|PrintString "three"))

(event EventBeginPlay
  (bind _outactors (Actor|GetAllActorsOfClass "/Script/LevelSequence.LevelSequenceActor"))
  (bind _output_get (Variables|Default|Setsequence (Utilities|Array|Get(acopy) _outactors)))
  (Class|LevelSequenceActor|SetEventReceivers _output_get (Utilities|Array|MakeArray self)))

(event Input|AxisEvents|InputAxisMoveFoward
  (params (AxisValue :type Float%20%28single-precision%29))
  (if (!= AxisValue 0.0)
    (Pawn|Input|AddMovementInput (Math|Rotator|GetRotationXVector (Math|Rotator|MakeRotator (.roll (Pawn|GetControlRotation :!class /Script/Engine.Pawn)) 0.0 0.0)) AxisValue false)))

(event Input|AxisEvents|InputAxisMoveUp
  (params (AxisValue :type Float%20%28single-precision%29))
  (if (!= AxisValue 0.0)
    (Pawn|Input|AddMovementInput (Math|Vector|GetUpVector (Math|Rotator|MakeRotator 0.0 0.0 (.yaw (Pawn|GetControlRotation :!class /Script/Engine.Pawn)))) AxisValue false)))

(event Input|AxisEvents|InputAxisMoveRight
  (params (AxisValue :type Float%20%28single-precision%29))
  (if (!= AxisValue 0.0)
    (Pawn|Input|AddMovementInput (Math|Vector|GetRightVector (Math|Rotator|MakeRotator 0.0 (.pitch (Pawn|GetControlRotation :!class /Script/Engine.Pawn)) 0.0)) AxisValue false)))

(event Input|KeyboardEvents|MotionControllerRightTrigger
  (params (Key :type Key%20Structure :default "AnyKey"))
  (:Pressed
    (Development|PrintString "右扳机")))

(event Input|KeyboardEvents|MotionControllerRightGrip1
  (params (Key :type Key%20Structure :default "AnyKey"))
  (:Pressed
    (Development|PrintString "右手柄1")))

(event Input|KeyboardEvents|MotionControllerRightGrip2
  (params (Key :type Key%20Structure :default "AnyKey"))
  (:Pressed
    (Development|PrintString "右手柄2")))

(event Input|KeyboardEvents|MotionControllerLeftTrigger
  (params (Key :type Key%20Structure :default "AnyKey"))
  (:Pressed
    (Development|PrintString "左扳机")))

(event Input|KeyboardEvents|MotionControllerLeftGrip1
  (params (Key :type Key%20Structure :default "AnyKey"))
  (:Pressed
    (Development|PrintString "左手柄1")))

(event Input|KeyboardEvents|MotionControllerLeftGrip2
  (params (Key :type Key%20Structure :default "AnyKey"))
  (:Pressed
    (Development|PrintString "左手柄2")))

(fn ConstructionScript)